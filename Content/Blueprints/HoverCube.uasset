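; HoverCube is an actor that pairs a Cube component with six HoverComponent3BP components, apparently to make the cube hover.
; On BeginPlay it sets the Cube as the TargetBody of every hover component, so all six share one body.
; The Blueprint has no other logic: Tick and the construction script are empty, leaving any hover behavior to the components.
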(event `self.ReceiveBeginPlay`
  (bind _cube (`self.Cube`))
  (set `/Game/Blueprints/HoverComponent3_BP.TargetBody` _cube (`self.HoverComponent3_BP`))
  (set `/Game/Blueprints/HoverComponent3_BP.TargetBody` _cube (`self.HoverComponent3_BP1`))
  (set `/Game/Blueprints/HoverComponent3_BP.TargetBody` _cube (`self.HoverComponent3_BP2`))
  (set `/Game/Blueprints/HoverComponent3_BP.TargetBody` _cube (`self.HoverComponent3_BP3`))
  (set `/Game/Blueprints/HoverComponent3_BP.TargetBody` _cube (`self.HoverComponent3_BP5`))
  (set `/Game/Blueprints/HoverComponent3_BP.TargetBody` _cube (`self.HoverComponent3_BP4`)))

(fn `UserConstructionScript`)