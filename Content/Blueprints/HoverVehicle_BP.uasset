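; Hover vehicle Blueprint that drives a physics car mesh on five hover components, four side ones and a center one, initialized with a shared trace length.
; MoveForward pushes the mesh along its forward vector.
; MoveRight applies yaw torque, inverted when reversing, and fakes body lean by lengthening the hover traces on the steered side.
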(event `self.ReceiveBeginPlay`
  (bind _output_get (set `self.HoverComponentsArray` (`|MakeArray` (`self.HoverComponent1`) (`self.HoverComponent3`) (`self.HoverComponent2`) (`self.HoverComponent4`) (`self.HoverComponent_Center`))))
  (for _array_element _output_get
    (`/Game/Blueprints/HoverComponent_BP.InitComponent` (`self.HoverComponentsArray`) (`self.CarMesh`))
    (set `/Game/Blueprints/HoverComponent_BP.TraceLength` (`self.HoverDistance`) _array_element)))

(event `InputAxis|MoveForward`
  (params (AxisValue :type "Float (single-precision)"))
  (bind _carmesh (`self.CarMesh`))
  (`PrimitiveComponent.AddForce` _carmesh (* (* (`SceneComponent.GetForwardVector` _carmesh) (`self.ForwardForce`)) AxisValue) "None" false))

(event `InputAxis|MoveRight`
  (params (AxisValue :type "Float (single-precision)"))
  (bind _lefthoverdistance (`self.LeftHoverDistance`))
  (bind _righthoverdistance (`self.RightHoverDistance`))
  (bind _hoverdistance (`self.HoverDistance`))
  (bind _carmesh (`self.CarMesh`))
  (bind _returnvalue (`KismetMathLibrary.FCeil` (`KismetMathLibrary.Abs` AxisValue)))
  (bind _returnvalue_2 (+ _hoverdistance (* _hoverdistance (* _returnvalue (`self.LeanAmount`)))))
  (if (> (* _returnvalue (`KismetMathLibrary.SignOfFloat` AxisValue)) 0.0)
    (set `self.LeftHoverDistance` _hoverdistance)
    (set `self.RightHoverDistance` _returnvalue_2)
    (else
      (set `self.RightHoverDistance` _hoverdistance)
      (set `self.LeftHoverDistance` _returnvalue_2)))
  (set `/Game/Blueprints/HoverComponent_BP.TraceLength` _lefthoverdistance (`self.HoverComponent1`))
  (set `/Game/Blueprints/HoverComponent_BP.TraceLength` _lefthoverdistance (`self.HoverComponent3`))
  (set `/Game/Blueprints/HoverComponent_BP.TraceLength` _righthoverdistance (`self.HoverComponent2`))
  (set `/Game/Blueprints/HoverComponent_BP.TraceLength` _righthoverdistance (`self.HoverComponent4`))
  (if (!= _returnvalue 0)
    (`PrimitiveComponent.AddTorque` (`self.CarMesh`) (* (`SceneComponent.GetUpVector` (`self.CarMesh`)) (* (* AxisValue (`KismetMathLibrary.SelectFloat` 1.0 -1.0 (> (`KismetMathLibrary.Dot_VectorVector` (`SceneComponent.GetComponentVelocity` _carmesh) (`SceneComponent.GetForwardVector` _carmesh)) -0.1))) (`self.TurnTorque`))) "None" false)))

(fn `UserConstructionScript`)