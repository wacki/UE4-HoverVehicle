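; HoverVehicle_BP_2 is a physics-driven hover vehicle that responds to forward input.
; BeginPlay enables simulation on CarMesh and passes it to HoverBoxComponentBP as its parent component.
; The MoveForward axis applies force along the mesh's forward vector.
; MoveRight is empty, and the torque steering logic, which flips direction when moving backward, is disconnected and never runs.
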(event `self.ReceiveBeginPlay`
  (`PrimitiveComponent.SetSimulatePhysics` (`self.CarMesh`) true)
  (set `/Game/Blueprints/HoverBoxComponent_BP.ParentComponent` (`self.CarMesh`) (`self.HoverBoxComponent_BP`)))

(event `InputAxis|MoveForward`
  (params (AxisValue :type "Float (single-precision)"))
  (bind _carmesh (`self.CarMesh`))
  (`PrimitiveComponent.AddForce` _carmesh (* (* (`SceneComponent.GetForwardVector` _carmesh) (`self.ForwardForce`)) AxisValue) "None" false))

(event `InputAxis|MoveRight`
  (params (AxisValue :type "Float (single-precision)")))

(fn `UserConstructionScript`)