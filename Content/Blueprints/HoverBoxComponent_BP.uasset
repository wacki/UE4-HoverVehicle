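; HoverBoxComponent is a scene component that applies a hover force to its parent component at its own location.
; Each tick it box-traces HoverDistance along its local down axis on the Visibility channel.
; It pushes along the impact normal, scaled by a Lerp from HoverForce to zero with HoverDistance divided by hit distance as alpha.
; The trace draws debug shapes and that ratio prints to screen.
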(event `self.ReceiveTick`
  (params (DeltaSeconds :type "Float (single-precision)"))
  (`|ExecutionSequence`
    (:`then_0`
      (set `self.TraceEndPos` (+ (`self.K2_GetComponentLocation`) (* (`self.GetUpVector`) (* -1 (`self.HoverDistance`))))))
    (:`then_1`
      (bind _outhit (`KismetSystemLibrary.BoxTraceSingle` :`Start` (`self.K2_GetComponentLocation`) :`End` (`self.TraceEndPos`) :`HalfSize` (50.0 50.0 50.0) :`Orientation` (`self.K2_GetComponentRotation`) :`TraceChannel` "TraceTypeQuery1" :`DrawDebugType` "ForOneFrame"))
      (bind (_bblockinghit _binitialoverlap _time _location _impactpoint _normal _impactnormal) (`GameplayStatics.BreakHitResult` _outhit))
      (bind _returnvalue (/ (`self.HoverDistance`) (`KismetMathLibrary.VSize` (- _impactpoint (`self.K2_GetComponentLocation`)))))
      (`PrimitiveComponent.AddForceAtLocation` (`self.ParentComponent`) (* _impactnormal (`KismetMathLibrary.Lerp` (`self.HoverForce`) 0.0 _returnvalue)) (`self.K2_GetComponentLocation`) "None")
      (`KismetSystemLibrary.PrintString` (`KismetStringLibrary.Conv_DoubleToString` _returnvalue)))))