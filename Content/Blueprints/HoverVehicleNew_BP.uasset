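; Player-driven hover vehicle Blueprint that moves by applying physics forces to its CarMesh, which it registers through SetVehicleMesh on BeginPlay.
; MoveForward stores the axis value and pushes the mesh along its forward vector, scaled by ForwardForce.
; MoveRight applies TurnTorque around the mesh's up vector, inverting steering while the stored forward input is negative.
; No hover logic appears in these graphs.
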(event `self.ReceiveBeginPlay`
  (`self.SetVehicleMesh` (`self.CarMesh`)))

(event `InputAxis|MoveForward`
  (params (AxisValue :type "Float (single-precision)"))
  (bind _carmesh (`self.CarMesh`))
  (bind _output_get (set `self.ForwardValue` AxisValue))
  (`PrimitiveComponent.AddForce` _carmesh (* (* (`SceneComponent.GetForwardVector` _carmesh) (`self.ForwardForce`)) _output_get) "None" false))

(event `InputAxis|MoveRight`
  (params (AxisValue :type "Float (single-precision)"))
  (`PrimitiveComponent.AddTorque` (`self.CarMesh`) (* (`SceneComponent.GetUpVector` (`self.CarMesh`)) (* (* AxisValue (`KismetMathLibrary.SelectFloat` -1.0 1.0 (< (`self.ForwardValue`) 0.0))) (`self.TurnTorque`))) "None" false))

(fn `UserConstructionScript`)