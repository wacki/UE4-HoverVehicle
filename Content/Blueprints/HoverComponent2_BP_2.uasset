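; Hover component that acts as a damped spring, applying force to a target body to hold it near a set hover distance above surfaces.
; Each Tick, it line-traces down world Z to twice that distance.
; On a hit, normalized height error drives stiffness and its frame-to-frame change drives damping, with force applied along the component's up vector.
; Debug trace drawing and printing of the compression ratio are left on.
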(event `self.ReceiveTick`
  (params (DeltaSeconds :type "Float (single-precision)"))
  (bind _returnvalue (/ (- (`self.HoverDistance`) (`KismetMathLibrary.VSize` (- (`self.ImpactLocation`) (`self.K2_GetComponentLocation`)))) (`self.HoverDistance`)))
  (set `self.DeltaSeconds` DeltaSeconds)
  (`|ExecutionSequence`
    (:`then_0`
      (set `self.TraceEndPos` (+ (`self.K2_GetComponentLocation`) (* (0.0 0.0 1.0) (* -2 (`self.HoverDistance`))))))
    (:`then_1`
      (bind (_outhit _returnvalue_2) (`KismetSystemLibrary.LineTraceSingle` :`Start` (`self.K2_GetComponentLocation`) :`End` (`self.TraceEndPos`) :`TraceChannel` "TraceTypeQuery1" :`DrawDebugType` "ForOneFrame"))
      (set `self.RaycastHit` _returnvalue_2)
      (bind (_bblockinghit _binitialoverlap _time _location _impactpoint _normal _impactnormal) (`GameplayStatics.BreakHitResult` _outhit))
      (set `self.ImpactNormal` _impactnormal)
      (set `self.ImpactLocation` _impactpoint))
    (:`then_2`
      (if (`self.RaycastHit`)
        (`|ExecutionSequence`
          (:`then_0`
            (set `self.ActualHeight` (- (`self.HoverDistance`) (`KismetMathLibrary.VSize` (- (`self.ImpactLocation`) (`self.K2_GetComponentLocation`)))))
            (set `self.SpringVelocity` (/ (- (`self.PrevActualHeight`) (`self.ActualHeight`)) (`self.DeltaSeconds`))))
          (:`then_1`
            (set `self.HoverForceVec` (* (`self.GetUpVector`) (- (* _returnvalue (`self.SpringStiffness`)) (* (`self.SpringDampening`) (`self.SpringVelocity`)))))
            (`KismetSystemLibrary.PrintString` (`KismetStringLibrary.Conv_DoubleToString` _returnvalue))
            (`PrimitiveComponent.AddForce` (`self.TargetBody`) (`self.HoverForceVec`) "None" false))
          (:`then_2`
            (set `self.PrevActualHeight` (`self.ActualHeight`))))))))