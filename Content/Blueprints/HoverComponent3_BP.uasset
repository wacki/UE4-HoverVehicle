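; Hover component that applies a damped spring force to TargetBody to float it above surfaces.
; Each tick it line-traces down its local axis and, on a hit, turns compression and its rate of change into a force along the up vector.
; IsMagnetic doubles the trace length, so the spring also pulls toward surfaces beyond hover distance.
; Debug trace drawing and spring-ratio printing are left on.
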(event `self.ReceiveTick`
  (params (DeltaSeconds :type "Float (single-precision)"))
  (bind _hoverdistance (`self.HoverDistance`))
  (bind _returnvalue (/ (`self.DistanceFromSurface`) (`self.HoverDistance`)))
  (set `self.DeltaSeconds` DeltaSeconds)
  (`|ExecutionSequence`
    (:`then_0`
      ;[1 1 1] Calculate trace destination
      (if (`self.IsMagnetic`)
        (set `self.TraceLength` (* -2 _hoverdistance))
        (else
          (set `self.TraceLength` (* -1 _hoverdistance))))
      (set `self.TraceEndPos` (+ (`self.K2_GetComponentLocation`) (* (`self.GetUpVector`) (`self.TraceLength`)))))
    (:`then_1`
      ;[1 1 1] Do the actual line trace and save out relevant information into variables
      (bind (_outhit _returnvalue_2) (`KismetSystemLibrary.LineTraceSingle` :`Start` (`self.K2_GetComponentLocation`) :`End` (`self.TraceEndPos`) :`TraceChannel` "TraceTypeQuery1" :`DrawDebugType` "ForOneFrame"))
      (set `self.RaycastHit` _returnvalue_2)
      (bind (_bblockinghit _binitialoverlap _time _location _impactpoint _normal _impactnormal) (`GameplayStatics.BreakHitResult` _outhit))
      (set `self.ImpactNormal` _impactnormal)
      (set `self.ImpactLocation` _impactpoint))
    (:`then_2`
      (if (`self.RaycastHit`)
        (`|ExecutionSequence`
          (:`then_0`
            ;[1 1 1] Update current spring velocity and distance from ground
            (set `self.DistanceFromSurface` (- (`self.HoverDistance`) (`KismetMathLibrary.VSize` (- (`self.ImpactLocation`) (`self.K2_GetComponentLocation`)))))
            (set `self.SpringVelocity` (/ (- (`self.PrevDistanceFromSurface`) (`self.DistanceFromSurface`)) (`self.DeltaSeconds`))))
          (:`then_1`
            ;[1 1 1] Calculate and apply damped spring hover force
            (set `self.HoverForceVec` (* (`self.GetUpVector`) (- (* _returnvalue (`self.SpringStiffness`)) (* (`self.SpringDampening`) (`self.SpringVelocity`)))))
            (`KismetSystemLibrary.PrintString` (`KismetStringLibrary.Conv_DoubleToString` _returnvalue))
            (`PrimitiveComponent.AddForce` (`self.TargetBody`) (`self.HoverForceVec`) "None" false))
          (:`then_2`
            ;[1 1 1] Set previous distance from surface var
            (set `self.PrevDistanceFromSurface` (`self.DistanceFromSurface`))))))))